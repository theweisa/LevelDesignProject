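; BP_Checkpoint is a trigger actor that records itself as the player's current checkpoint when touched.
; On overlap it casts to BP_Player and, if it is not already that player's CurrentCheckpoint, calls EnterCheckpoint.
; That event stores the checkpoint on the player, prints a message and disables the Box collision, so the trigger fires only once.
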(event `self.ReceiveActorBeginOverlap`
  (params (OtherActor :type "Actor Object Reference"))
  (bind _asbp_player (cast `/Game/Blueprints/BP_Player` OtherActor))
  (if (!= (`/Game/Blueprints/BP_Player.currentCheckpoint` _asbp_player) self)
    (`self.EnterCheckpoint` _asbp_player)))

(event `EnterCheckpoint`
  (params (player :type "/Game/Blueprints/BP_Player Object Reference"))
  (set `/Game/Blueprints/BP_Player.currentCheckpoint` self player)
  (`KismetSystemLibrary.PrintString` "new checkpoint!")
  (`PrimitiveComponent.SetCollisionEnabled` (`self.Box`) "NoCollision"))

(fn `UserConstructionScript`)