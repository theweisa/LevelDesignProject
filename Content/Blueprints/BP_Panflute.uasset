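; BP_Panflute is an actor that makes a timed round trip when the player enters its box trigger.
; An overlap by BP_Player starts the move unless one is already running, tracked by a Moving flag.
; Chained linear vector tweens slide it to a fixed world X, pause briefly, then return it to the location saved at BeginPlay, without sweeping.
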(event `self.ReceiveBeginPlay`
  (set `self.basePosition` (`self.K2_GetActorLocation`)))

(event `MoveFlute`
  (bind (_returnvalue_x _returnvalue_y _returnvalue_z) (`KismetMathLibrary.BreakVector` (`self.K2_GetActorLocation`)))
  (set `self.moving` true)
  (bind (_asynctaskproxy _value) (`FCTweenBPActionVector.TweenVector` (`self.K2_GetActorLocation`) (`KismetMathLibrary.MakeVector` 6090.0 _returnvalue_y _returnvalue_z) 10.0 "Linear")
    (:`ApplyEasing`
      (`self.K2_SetActorLocation` _value))
    (:`OnComplete`
      (`KismetSystemLibrary.Delay` 4.0)
      (bind (_asynctaskproxy_2 _value_2) (`FCTweenBPActionVector.TweenVector` (`self.K2_GetActorLocation`) (`self.basePosition`) 10.0 "Linear")
        (:`ApplyEasing`
          (`self.K2_SetActorLocation` _value_2))
        (:`OnComplete`
          (set `self.moving` false))))))

(event `self.Box.OnComponentBeginOverlap`
  (params (OverlappedComponent :type "PrimitiveComponent Object Reference") (OtherActor :type "Actor Object Reference") (OtherComp :type "PrimitiveComponent Object Reference") (OtherBodyIndex :type Integer) (bFromSweep :type Boolean) (SweepResult :type "HitResult Structure (by ref)"))
  (cast `/Game/Blueprints/BP_Player` OtherActor)
  (if (not (`self.moving`))
    (`self.MoveFlute`)))

(fn `UserConstructionScript`)