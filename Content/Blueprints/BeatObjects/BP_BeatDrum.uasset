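; A beat-driven drum that alternates between winding up and knocking the player away on successive BeatEvent calls.
; Wind-up tweens its X/Y scale inward over most of MusicManager's beat interval; launch snaps it wider and tweens back to the base scale.
; The launch pushes BP_Player along the horizontal components of the drum-to-player direction, with no range check, and the first launch beat is skipped.
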(event `self.ReceiveBeginPlay`
  (`parent.ReceiveBeginPlay`)
  (set `self.baseScale` (`self.GetActorScale3D`)))

(event `self.BeatEvent`
  (params (beatInterval :type Integer))
  (`|ExecutionSequence`
    (:`then_0`
      (if (`self.windUp`)
        (if (`self.skipFirstBeat`)
          (`self.LaunchPlayer`)
          (else
            (set `self.skipFirstBeat` true)))
        (else
          (`self.WindDrum`))))
    (:`then_1`
      (set `self.windUp` (not (`self.windUp`))))))

(event `WindDrum`
  (bind (_basescale_x _basescale_y _basescale_z) (`KismetMathLibrary.BreakVector` (`self.baseScale`)))
  (bind (_asynctaskproxy _value) (`FCTweenBPActionVector.TweenVector` (`self.baseScale`) (`KismetMathLibrary.MakeVector` (.x (* (`KismetMathLibrary.MakeVector` _basescale_x _basescale_y _basescale_z) 0.9)) (.y (* (`KismetMathLibrary.MakeVector` _basescale_x _basescale_y _basescale_z) 0.9)) _basescale_z) (* (`/Game/Blueprints/MusicManager.beatInterval` (`self.musicManager`)) 0.8) "Linear")
    (:`ApplyEasing`
      (`self.SetActorScale3D` _value))))

(event `LaunchPlayer`
  (bind (_basescale_x _basescale_y _basescale_z) (`KismetMathLibrary.BreakVector` (`self.baseScale`)))
  (`|ExecutionSequence`
    (:`then_0`
      (bind (_asynctaskproxy _value) (`FCTweenBPActionVector.TweenVector` (`KismetMathLibrary.MakeVector` (.x (* (`KismetMathLibrary.MakeVector` _basescale_x _basescale_y _basescale_z) 1.1)) (.y (* (`KismetMathLibrary.MakeVector` _basescale_x _basescale_y _basescale_z) 1.1)) _basescale_z) (`self.baseScale`) 0.5 "Linear")
        (:`ApplyEasing`
          (`self.SetActorScale3D` _value))))
    (:`then_1`
      (bind _returnvalue (`GameplayStatics.GetActorOfClass` "/Game/Blueprints/BP_Player.BP_Player_C"))
      (`/Engine/EditorBlueprintResources/StandardMacros.IsValid` _returnvalue
        (:`Is Valid`
          (bind _returnvalue_2 (`KismetMathLibrary.GetDirectionUnitVector` (`self.K2_GetActorLocation`) (`self.K2_GetActorLocation` _returnvalue)))
          (`KismetSystemLibrary.PrintString` (`KismetStringLibrary.Conv_VectorToString` _returnvalue_2) true true (struct :`G` 0.66 :`B` 1.0 :`A` 1.0) 10.0)
          (bind (_returnvalue_x _returnvalue_y) (`KismetMathLibrary.BreakVector` (* _returnvalue_2 (`self.launchForce`))))
          (`Character.LaunchCharacter` _returnvalue (`KismetMathLibrary.MakeVector` _returnvalue_x _returnvalue_y) false false))))))

(fn `UserConstructionScript`
  (`parent.UserConstructionScript`))