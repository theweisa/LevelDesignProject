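; A beat-driven platform that alternates between present and absent each time its beat event fires.
; On BeginPlay it caches the static mesh's collision setting and applies the initial Visible state.
; Each BeatEvent flips Visible, and ToggleActive then shows the actor with its cached collision or hides it with collision disabled.
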(event `self.ReceiveBeginPlay`
  (`parent.ReceiveBeginPlay`)
  (set `self.collisionType` (`PrimitiveComponent.GetCollisionEnabled` (`self.StaticMesh`)))
  (`self.ToggleActive` (`self.visible`)))

(event `self.BeatEvent`
  (params (beatInterval :type Integer))
  (bind _output_get (set `self.visible` (not (`self.visible`))))
  (`self.ToggleActive` _output_get))

(fn `ToggleActive`
  (params (active :type Boolean))
  (if active
    (`self.SetActorHiddenInGame` false)
    (`PrimitiveComponent.SetCollisionEnabled` (`self.StaticMesh`) (`self.collisionType`))
    (else
      (`self.SetActorHiddenInGame` true)
      (`PrimitiveComponent.SetCollisionEnabled` (`self.StaticMesh`) "NoCollision"))))

(fn `UserConstructionScript`
  (`parent.UserConstructionScript`))