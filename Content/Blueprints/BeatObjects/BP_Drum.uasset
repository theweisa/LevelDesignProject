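; BP_Drum is a beat-driven launch pad that alternates between winding up and launching players on successive BeatEvent calls.
; The wind-up tweens its X/Y scale down, while the launch starts it enlarged and eases back to base scale.
; On launch, BP_Player pawns overlapping its Box are launched along the drum's up vector, using SuperLaunchForce if falling and NormalLaunchForce otherwise.
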(event `self.ReceiveBeginPlay`
  (`parent.ReceiveBeginPlay`)
  (set `self.baseScale` (`self.GetActorScale3D`)))

(event `self.ReceiveTick`
  (params (DeltaSeconds :type "Float (single-precision)"))
  (`parent.ReceiveTick` DeltaSeconds))

(event `self.BeatEvent`
  (params (beatInterval :type Integer))
  (`|ExecutionSequence`
    (:`then_0`
      (if (`self.windUp`)
        (`self.LaunchPlayer`)
        (else
          (`self.WindDrum`))))
    (:`then_1`
      (set `self.windUp` (not (`self.windUp`))))))

(event `WindDrum`
  (bind (_basescale_x _basescale_y _basescale_z) (`KismetMathLibrary.BreakVector` (`self.baseScale`)))
  (bind (_asynctaskproxy _value) (`FCTweenBPActionVector.TweenVector` (`self.baseScale`) (`KismetMathLibrary.MakeVector` (.x (* (`KismetMathLibrary.MakeVector` _basescale_x _basescale_y _basescale_z) 0.9)) (.y (* (`KismetMathLibrary.MakeVector` _basescale_x _basescale_y _basescale_z) 0.9)) _basescale_z) 0.33 "OutExpo")
    (:`ApplyEasing`
      (`self.SetActorScale3D` _value))))

(event `LaunchPlayer`
  (bind _box (`self.Box`))
  (bind (_basescale_x _basescale_y _basescale_z) (`KismetMathLibrary.BreakVector` (`self.baseScale`)))
  (`|ExecutionSequence`
    (:`then_0`
      (bind (_asynctaskproxy _value) (`FCTweenBPActionVector.TweenVector` (`KismetMathLibrary.MakeVector` (.x (* (`KismetMathLibrary.MakeVector` _basescale_x _basescale_y _basescale_z) 1.1)) (.y (* (`KismetMathLibrary.MakeVector` _basescale_x _basescale_y _basescale_z) 1.1)) _basescale_z) (`self.baseScale`) 0.5 "Linear")
        (:`ApplyEasing`
          (`self.SetActorScale3D` _value))))
    (:`then_1`
      (bind (_outactors _returnvalue) (`KismetSystemLibrary.ComponentOverlapActors` _box (`SceneComponent.K2_GetComponentToWorld` _box) (`|MakeArray` "ObjectTypeQuery3" :!type "EObjectTypeQuery Enum") "/Game/Blueprints/BP_Player.BP_Player_C"))
      (if _returnvalue
        (for _array_element _outactors
          (bind _asbp_player (cast `/Game/Blueprints/BP_Player` _array_element))
          (if (`NavMovementComponent.IsFalling` (`Character.CharacterMovement` _asbp_player))
            (`Character.LaunchCharacter` _asbp_player (* (`self.GetActorUpVector`) (`self.superLaunchForce`)) false false)
            (else
              (`Character.LaunchCharacter` _asbp_player (* (`self.GetActorUpVector`) (`self.normalLaunchForce`)) false false))))))))

(fn `UserConstructionScript`
  (`parent.UserConstructionScript`))