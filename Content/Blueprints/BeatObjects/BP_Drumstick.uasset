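; Beat-driven drumstick hazard that swings on each beat and kills the player it strikes.
; BeatEvent alternates between raising the stick to a set pitch and dropping it back to its starting rotation.
; Rotation tweens shape the motion, easing in on the lift and bouncing out on the drop.
; The capsule collides only during the downswing, calling OnDeath on an overlapping BP_Player.
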(event `self.ReceiveBeginPlay`
  (`parent.ReceiveBeginPlay`)
  (set `self.baseRotation` (`self.K2_GetActorRotation`))
  (`PrimitiveComponent.SetCollisionEnabled` (`self.Capsule`) "NoCollision"))

(event `self.BeatEvent`
  (params (beatInterval :type Integer))
  (`|ExecutionSequence`
    (:`then_0`
      (if (`self.drumstickDown`)
        (`self.StickUp`)
        (else
          (`self.StickDown`))))
    (:`then_1`
      (set `self.drumstickDown` (not (`self.drumstickDown`))))))

(event `StickUp`
  (bind (_baserotation_roll _baserotation_pitch _baserotation_yaw) (`KismetMathLibrary.BreakRotator` (`self.baseRotation`)))
  (`|ExecutionSequence`
    (:`then_0`
      (bind (_asynctaskproxy _value) (`FCTweenBPActionRotator.TweenRotator` (`self.K2_GetActorRotation`) (`KismetMathLibrary.MakeRotator` _baserotation_roll (`self.toRotationAngle`) _baserotation_yaw) 1.0 "InQuart")
        (:`ApplyEasing`
          (`self.K2_SetActorRotation` _value))))))

(event `StickDown`
  (`|ExecutionSequence`
    (:`then_0`
      (bind (_asynctaskproxy _value) (`FCTweenBPActionRotator.TweenRotator` (`self.K2_GetActorRotation`) (`self.baseRotation`) 1.0 "OutBounce")
        (:`ApplyEasing`
          (`self.K2_SetActorRotation` _value))
        (:`OnComplete`
          (`PrimitiveComponent.SetCollisionEnabled` (`self.Capsule`) "NoCollision"))))
    (:`then_1`
      (`PrimitiveComponent.SetCollisionEnabled` (`self.Capsule`) "QueryAndPhysics"))))

(event `self.Capsule.OnComponentBeginOverlap`
  (params (OverlappedComponent :type "PrimitiveComponent Object Reference") (OtherActor :type "Actor Object Reference") (OtherComp :type "PrimitiveComponent Object Reference") (OtherBodyIndex :type Integer) (bFromSweep :type Boolean) (SweepResult :type "HitResult Structure (by ref)"))
  (bind _asbp_player (cast `/Game/Blueprints/BP_Player` OtherActor))
  (`/Game/Blueprints/BP_Player.OnDeath` _asbp_player))

(fn `UserConstructionScript`
  (`parent.UserConstructionScript`))