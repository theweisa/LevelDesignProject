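; BP_PushDrum is a beat-driven drum that launches players standing in its box whenever its beat event fires.
; Each beat tweens the actor from an enlarged X and Z scale back to the scale stored at BeginPlay, giving a pulse.
; The same beat queries the box for overlapping BP_Player pawns and launches them along the drum's right vector times LaunchForce plus PushInfluence, overriding their current velocity.
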(event `self.ReceiveBeginPlay`
  (`parent.ReceiveBeginPlay`)
  (set `self.baseScale` (`self.GetActorScale3D`)))

(event `self.BeatEvent`
  (params (beatInterval :type Integer))
  (bind _box (`self.Box`))
  (bind (_basescale_x _basescale_y) (`KismetMathLibrary.BreakVector` (`self.baseScale`)))
  (bind _basescale (`self.baseScale`))
  (`|ExecutionSequence`
    (:`then_0`
      (bind (_asynctaskproxy _value) (`FCTweenBPActionVector.TweenVector` (`KismetMathLibrary.MakeVector` (.x (* _basescale 1.1)) _basescale_y (.z (* _basescale 1.1))) _basescale 0.3 "Linear")
        (:`ApplyEasing`
          (`self.SetActorScale3D` _value))))
    (:`then_1`
      (bind (_outactors _returnvalue) (`KismetSystemLibrary.ComponentOverlapActors` _box (`SceneComponent.K2_GetComponentToWorld` _box) (`|MakeArray` "ObjectTypeQuery3" :!type "EObjectTypeQuery Enum") "/Game/Blueprints/BP_Player.BP_Player_C"))
      (if _returnvalue
        (for _array_element _outactors
          (bind _asbp_player (cast `/Game/Blueprints/BP_Player` _array_element))
          (`Character.LaunchCharacter` _asbp_player (+ (* (`self.GetActorRightVector`) (`self.launchForce`)) (`self.pushInfluence`)) true true))))))

(fn `UserConstructionScript`
  (`parent.UserConstructionScript`))