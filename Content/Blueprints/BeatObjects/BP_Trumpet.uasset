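; BP_Trumpet is a beat-driven trumpet that alternates between winding up and launching the player on successive BeatEvents.
; Winding up tweens the actor down from its base scale, then launching snaps it oversized and tweens it back, with both durations scaled to the MusicManager beat interval.
; On launch, any BP_Player inside the Box is thrown along the actor's forward vector plus an additional velocity, overriding current velocity.
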(event `self.ReceiveBeginPlay`
  (`parent.ReceiveBeginPlay`)
  (set `self.baseScale` (`self.GetActorScale3D`)))

(event `self.ReceiveTick`
  (params (DeltaSeconds :type "Float (single-precision)"))
  (`parent.ReceiveTick` DeltaSeconds))

(event `self.BeatEvent`
  (params (beatInterval :type Integer))
  (if (`self.windUp`)
    (`self.LaunchPlayer`)
    (else
      (`self.WindTrumpet`))))

(event `WindTrumpet`
  (set `self.windUp` true)
  (bind (_asynctaskproxy _value) (`FCTweenBPActionVector.TweenVector` (`self.GetActorScale3D`) (* (`self.baseScale`) 0.8) (* (`/Game/Blueprints/MusicManager.beatInterval` (`self.musicManager`)) 1.8) "OutQuart")
    (:`ApplyEasing`
      (`self.SetActorScale3D` _value))))

(event `LaunchPlayer`
  (bind _box (`self.Box`))
  (set `self.windUp` false)
  (`|ExecutionSequence`
    (:`then_0`
      (bind (_asynctaskproxy _value) (`FCTweenBPActionVector.TweenVector` (* (`self.baseScale`) 1.35) (`self.baseScale`) (* (`/Game/Blueprints/MusicManager.beatInterval` (`self.musicManager`)) 0.4) "Linear")
        (:`ApplyEasing`
          (`self.SetActorScale3D` _value))))
    (:`then_1`
      (bind (_outactors _returnvalue) (`KismetSystemLibrary.ComponentOverlapActors` _box (`SceneComponent.K2_GetComponentToWorld` _box) (`|MakeArray` "ObjectTypeQuery3" :!type "EObjectTypeQuery Enum") "/Game/Blueprints/BP_Player.BP_Player_C"))
      (if _returnvalue
        (for _array_element _outactors
          (bind _asbp_player (cast `/Game/Blueprints/BP_Player` _array_element))
          (`Character.LaunchCharacter` _asbp_player (+ (* (`self.GetActorForwardVector`) (`self.launchForce`)) (`self.additionalLaunchVelocity`)) true true))))))

(fn `NewFunction`)

(fn `UserConstructionScript`
  (`parent.UserConstructionScript`))