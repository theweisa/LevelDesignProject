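; Card is a beat object that moves to the next of four point actors each time BeatEvent fires, looping back to the first.
; Each step tweens location over TweenTime and, if ApplyRotation is set, tweens rotation toward the point's forward vector.
; The current index picks the target point and advances after the tweens start.
; On BeginPlay, the decal is hidden when HasShadow is off.
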(event `self.ReceiveTick`
  (params (DeltaSeconds :type "Float (single-precision)"))
  (`parent.ReceiveTick` DeltaSeconds))

(event `self.ReceiveBeginPlay`
  (`parent.ReceiveBeginPlay`)
  (if (not (`self.hasShadow`))
    (`SceneComponent.SetVisibility` (`self.Decal`) false false)))

(event `self.BeatEvent`
  (params (beatInterval :type Integer))
  (switch `int` (`self.currentPosIndex`)
    (:`0`
      (set `self.currentPointPos` (`self.K2_GetActorLocation` (`self.point0`)))
      (set `self.currentPointRot` (`KismetMathLibrary.Conv_RotatorToVector` (`self.K2_GetActorRotation` (`self.point0`)))))
    (:`1`
      (set `self.currentPointPos` (`self.K2_GetActorLocation` (`self.point1`)))
      (set `self.currentPointRot` (`KismetMathLibrary.Conv_RotatorToVector` (`self.K2_GetActorRotation` (`self.point1`)))))
    (:`2`
      (set `self.currentPointPos` (`self.K2_GetActorLocation` (`self.point2`)))
      (set `self.currentPointRot` (`KismetMathLibrary.Conv_RotatorToVector` (`self.K2_GetActorRotation` (`self.point2`)))))
    (:`3`
      (set `self.currentPointPos` (`self.K2_GetActorLocation` (`self.point3`)))
      (set `self.currentPointRot` (`KismetMathLibrary.Conv_RotatorToVector` (`self.K2_GetActorRotation` (`self.point3`))))))
  (`|ExecutionSequence`
    (:`then_0`
      (bind (_asynctaskproxy _value) (`FCTweenBPActionVector.TweenVector` (`self.K2_GetActorLocation`) (`self.currentPointPos`) (`self.tweenTime`))
        (:`ApplyEasing`
          (`self.K2_SetActorLocation` _value))))
    (:`then_1`
      (if (`self.applyRotation`)
        (bind (_asynctaskproxy_2 _value_2) (`FCTweenBPActionRotator.TweenRotator` (`self.K2_GetActorRotation`) (`KismetMathLibrary.Conv_VectorToRotator` (`self.currentPointRot`)) (`self.tweenTime`))
          (:`ApplyEasing`
            (`self.K2_SetActorRotation` _value_2)))))
    (:`then_2`
      (switch `int` (`self.currentPosIndex`)
        (:`0`
          (set `self.currentPosIndex` 1))
        (:`1`
          (set `self.currentPosIndex` 2))
        (:`2`
          (set `self.currentPosIndex` 3))
        (:`3`
          (set `self.currentPosIndex` 0))))))

(fn `UserConstructionScript`
  (`parent.UserConstructionScript`))