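; TestBeatObject is a test beat-reactive actor whose cube hops up or down on each BeatEvent.
; Each call flips a GoingUp flag and tweens the cube's world location a fixed distance along Z in the matching direction.
; The short TweenVector uses OutExpo easing for a snappy move, starting from the cube's current location rather than a stored origin.
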(event `self.BeatEvent`
  (params (beatInterval :type Integer))
  (bind _returnvalue (`SceneComponent.K2_GetComponentLocation` (`self.Cube`)))
  (bind _returnvalue_2 (`SceneComponent.K2_GetComponentLocation` (`self.Cube`)))
  (bind _output_get (set `self.goingUp` (not (`self.goingUp`))))
  (if _output_get
    (bind (_asynctaskproxy _value) (`FCTweenBPActionVector.TweenVector` _returnvalue_2 (`KismetMathLibrary.MakeVector` (.x _returnvalue_2) (.y _returnvalue_2) (+ (.z _returnvalue_2) 50.0)) 0.3 "OutExpo")
      (:`ApplyEasing`
        (`SceneComponent.K2_SetWorldLocation` (`self.Cube`) _value false false)))
    (else
      (bind (_asynctaskproxy_2 _value_2) (`FCTweenBPActionVector.TweenVector` _returnvalue (`KismetMathLibrary.MakeVector` (.x _returnvalue) (.y _returnvalue) (+ (.z _returnvalue) -50.0)) 0.3 "OutExpo")
        (:`ApplyEasing`
          (`SceneComponent.K2_SetWorldLocation` (`self.Cube`) _value_2 false false))))))

(fn `UserConstructionScript`
  (`parent.UserConstructionScript`))