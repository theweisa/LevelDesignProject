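; WhiteKey is a beat object, a piano-style key that dips on BeatEvent and launches the player standing on it.
; BeatEvent tweens the actor down by KeyDown, then after a delay tweens it back to the location saved at BeginPlay.
; As the return starts, it launches the BP_Player tracked by the Box overlap, using LaunchForce vertically and the up vector scaled by YLaunchForce on Y.
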(event `self.ReceiveBeginPlay`
  (`parent.ReceiveBeginPlay`)
  (set `self.baseLocation` (`self.K2_GetActorLocation`)))

(event `self.BeatEvent`
  (params (beatInterval :type Integer))
  (bind (_returnvalue_x _returnvalue_y) (`KismetMathLibrary.BreakVector` (`self.GetActorUpVector`)))
  (bind (_returnvalue_x_2 _returnvalue_y_2 _returnvalue_z) (`KismetMathLibrary.BreakVector` (`self.K2_GetActorLocation`)))
  (bind _playerref (`self.playerRef`))
  (bind (_asynctaskproxy _value) (`FCTweenBPActionVector.TweenVector` (`self.K2_GetActorLocation`) (`KismetMathLibrary.MakeVector` _returnvalue_x_2 _returnvalue_y_2 (- _returnvalue_z (`self.keyDown`))) (`self.tweenTime`))
    (:`then`
      (set `self.isKeyUp` false))
    (:`ApplyEasing`
      (`self.K2_SetActorLocation` _value)
      (`KismetSystemLibrary.Delay` (`self.tweenTime`))
      (`|ExecutionSequence`
        (:`then_0`
          (bind (_asynctaskproxy_2 _value_2) (`FCTweenBPActionVector.TweenVector` (`self.K2_GetActorLocation`) (`self.baseLocation`) (`self.tweenTime`))
            (:`ApplyEasing`
              (`self.K2_SetActorLocation` _value_2)
              (set `self.isKeyUp` true))))
        (:`then_1`
          (`/Engine/EditorBlueprintResources/StandardMacros.IsValid` _playerref
            (:`Is Valid`
              (`Character.LaunchCharacter` _playerref (`KismetMathLibrary.MakeVector` _returnvalue_x (* _returnvalue_y (`self.yLaunchForce`)) (`self.launchForce`)) false true))))))))

(event `self.Box.OnComponentBeginOverlap`
  (params (OverlappedComponent :type "PrimitiveComponent Object Reference") (OtherActor :type "Actor Object Reference") (OtherComp :type "PrimitiveComponent Object Reference") (OtherBodyIndex :type Integer) (bFromSweep :type Boolean) (SweepResult :type "HitResult Structure (by ref)"))
  (bind _asbp_player (cast `/Game/Blueprints/BP_Player` OtherActor))
  (set `self.playerRef` _asbp_player))

(event `self.Box.OnComponentEndOverlap`
  (params (OverlappedComponent :type "PrimitiveComponent Object Reference") (OtherActor :type "Actor Object Reference") (OtherComp :type "PrimitiveComponent Object Reference") (OtherBodyIndex :type Integer))
  (cast `/Game/Blueprints/BP_Player` OtherActor)
  (set `self.playerRef` null))

(fn `UserConstructionScript`
  (`parent.UserConstructionScript`))