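; Music manager actor that acts as a BPM-driven beat clock for every BP_BeatObject in the level.
; BeginPlay derives the beat interval from Bpm and caches those actors.
; While SongStarted is true, Tick accumulates delta time into SongPosition rather than reading audio playback.
; Each new beat calls IncrementMeasure on the objects, and MeasureInterval subdivisions within it call CheckBeat, both with debug prints.
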(event `self.ReceiveBeginPlay`
  (set `self.beatInterval` (/ 60.0 (`self.bpm`)))
  (bind _outactors (`GameplayStatics.GetAllActorsOfClass` "/Game/Blueprints/BeatObjects/BP_BeatObject.BP_BeatObject_C"))
  (set `self.beatObjects` _outactors))

(event `self.ReceiveTick`
  (params (DeltaSeconds :type "Float (single-precision)"))
  (if (`self.songStarted`)
    (set `self.songPosition` (+ DeltaSeconds (`self.songPosition`)))
    (`self.CheckBPM`)
    (`self.CheckMeasurePosition`)))

(fn `CheckBPM`
  (if (>= (`self.songPosition`) (* (`self.beatInterval`) (+ (`self.numBeatsIn`) 1)))
    (set `self.numBeatsIn` (+ (`self.numBeatsIn`) 1))
    (set `self.measurePosition` 0)
    (`KismetSystemLibrary.PrintString` "beat")
    (for _array_element (`self.beatObjects`)
      (`/Game/Blueprints/BeatObjects/BP_BeatObject.IncrementMeasure` _array_element))))

(fn `CheckMeasurePosition`
  (bind _beatinterval (`self.beatInterval`))
  (if (>= (`self.songPosition`) (+ (* (/ (`KismetMathLibrary.Conv_IntToDouble` (`self.measurePosition`)) (`KismetMathLibrary.Conv_IntToDouble` (`self.measureInterval`))) _beatinterval) (* _beatinterval (`self.numBeatsIn`))))
    (`|ExecutionSequence`
      (:`then_0`
        (for _array_element (`self.beatObjects`)
          (`/Game/Blueprints/BeatObjects/BP_BeatObject.CheckBeat` _array_element (`self.measurePosition`))))
      (:`then_1`
        (`KismetSystemLibrary.PrintString` (`KismetStringLibrary.Conv_IntToString` (`self.measurePosition`)) true true (struct :`G` 0.66 :`B` 1.0 :`A` 1.0) 10.0))
      (:`then_2`
        (bind _output_get (set `self.measurePosition` (+ (`self.measurePosition`) 1)))
        (if (> _output_get (`self.measureInterval`))
          (set `self.measurePosition` 0))))))

(fn `UserConstructionScript`)